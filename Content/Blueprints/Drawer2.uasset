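; Drawer2 is a grabbable VR drawer that slides along a single axis as the motion controller holding it moves.
; Grabbing stores the controller and starts a looping 0.01-second timer calling UpdateLocation, and dropping stops it.
; UpdateLocation adds the controller's X offset in Capsule space to the Capsule's relative X, clamped between the local X positions of the Spline's first two points.
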(event `self.GrabComponent.OnGrabbed`
  (params (`Motion Controller` :type "MotionControllerComponent Object Reference"))
  (set `self.Motion Controller` `Motion Controller`)
  (bind _returnvalue (`KismetSystemLibrary.K2_SetTimer` null "UpdateLocation" 0.01 true))
  (set `self.Timer` _returnvalue))

(event `self.GrabComponent.OnDropped`
  (`KismetSystemLibrary.K2_ClearAndInvalidateTimerHandle` (`self.Timer`))
  (set `self.Motion Controller` null))

(fn `UpdateLocation`
  (bind _capsule (`self.Capsule`))
  (bind _spline (`self.Spline`))
  (bind _returnvalue_x (`KismetMathLibrary.BreakVector` (`SplineComponent.GetLocationAtSplinePoint` _spline 1 "Local")))
  (bind _returnvalue_x_2 (`KismetMathLibrary.BreakVector` (`SplineComponent.GetLocationAtSplinePoint` _spline 0 "Local")))
  (bind (_relativelocation_x _relativelocation_y _relativelocation_z) (`KismetMathLibrary.BreakVector` (`SceneComponent.RelativeLocation` _capsule)))
  (`SceneComponent.K2_SetRelativeLocation` _capsule (`KismetMathLibrary.MakeVector` (`KismetMathLibrary.FClamp` (+ (.x (.location (`KismetMathLibrary.MakeRelativeTransform` (`SceneComponent.K2_GetComponentToWorld` (`self.Motion Controller`)) (`SceneComponent.K2_GetComponentToWorld` (`self.Capsule`))))) _relativelocation_x) _returnvalue_x_2 _returnvalue_x) _relativelocation_y _relativelocation_z) false false))

(fn `UserConstructionScript`)