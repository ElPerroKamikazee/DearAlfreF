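; Actor Blueprint for a prop, apparently a chair judging by its material, that dissolves away when a VRPawn enters its trigger box.
; On overlap it creates a dynamic instance of the chair material, applies it to the static mesh, and a timeline drives the DissolveAmount parameter.
; It also attaches the BP_Dissolve_System effect to the mesh and destroys the actor after a short delay.
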(event `self.Box.OnComponentBeginOverlap`
  (params (OverlappedComponent :type "PrimitiveComponent Object Reference") (OtherActor :type "Actor Object Reference") (OtherComp :type "PrimitiveComponent Object Reference") (OtherBodyIndex :type Integer) (bFromSweep :type Boolean) (SweepResult :type "HitResult Structure (by ref)"))
  (cast `/Game/VRTemplate/Blueprints/VRPawn` OtherActor)
  (`|ExecutionSequence`
    (:`then_0`
      (bind _returnvalue (`KismetMaterialLibrary.CreateDynamicMaterialInstance` "/Game/Dissolve/M_Chair_Default1_Inst.M_Chair_Default1_Inst"))
      (set `self.NewVar` _returnvalue))
    (:`then_1`
      (`PrimitiveComponent.SetMaterial` (`self.StaticMesh`) 0 (`self.NewVar`)))
    (:`then_2`
      (bind (_direction _newtrack_0) (`Timeline|Timeline`)
        (:`Update`
          (`MaterialInstanceDynamic.SetScalarParameterValue` (`self.NewVar`) "DissolveAmount" _newtrack_0))))
    (:`then_3`
      (`NiagaraFunctionLibrary.SpawnSystemAttached` "/Game/Dissolve/BP_Dissolve_System.BP_Dissolve_System" (`self.StaticMesh`) "None" (0.0 0.0 0.0) (struct) "SnapToTarget")
      (`KismetSystemLibrary.Delay` 3.0)
      (`self.K2_DestroyActor`))))

(fn `UserConstructionScript`)